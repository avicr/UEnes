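; Demo actor that runs an NES emulator in the world, playing a ROM on a cube screen with sound.
; BeginPlay feeds the emulator's screen texture into a dynamic material and its sound stream into an audio component, then optionally hands control to the local player.
; SetPlayer blends the view to this actor and enables input, mapping gamepad and keyboard to pad 0.
; Escape returns view to the pawn; R toggles render-thread video updates.
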(event `self.ReceiveBeginPlay`
  (bind _nes (`self.Nes`))
  (bind _audio (`self.Audio`))
  ;[1 1 1] Create dynamic material and set screen texture
  (bind _returnvalue (`PrimitiveComponent.CreateDynamicMaterialInstance` (`self.Cube`) 0 "/UEnes/M_UEnesScreen.M_UEnesScreen" "None"))
  (`MaterialInstanceDynamic.SetTextureParameterValue` _returnvalue "Texture" (`NesComponent.ScreenTexture` (`self.Nes`)))
  ;[1 1 1] Load ROM
  (`NesComponent.PlayFromFile` _nes (`self.RomPath`))
  (set `AudioComponent.Sound` (`NesComponent.NesSoundStream` _nes) _audio)
  (`AudioComponent.Play` _audio 0.0)
  ;[1 1 1] Set the player controller
  (if (`self.bAutoSetPlayer`)
    (`self.SetPlayer` (`GameplayStatics.GetPlayerControllerFromID` 0))))

(event `Key|Gamepad_Special_Right`
  (params (Key :type "Key Structure"))
  (bind _nes (`self.Nes`))
  ;[1 1 1] Input
  (:`Pressed`
    (`NesComponent.SetPadButtonState` _nes 0 "START" true :!label _label))
  (:`Released`
    (`NesComponent.SetPadButtonState` _nes 0 "START" false :!label _label_2)))

(event `Key|Enter`
  (params (Key :type "Key Structure"))
  ;[1 1 1] Input
  (:`Pressed`
    (goto _label))
  (:`Released`
    (goto _label_2)))

(event `Key|Gamepad_FaceButton_Bottom`
  (params (Key :type "Key Structure"))
  (bind _nes (`self.Nes`))
  ;[1 1 1] Input
  (:`Pressed`
    (`NesComponent.SetPadButtonState` _nes 0 "A" true :!label _label_3))
  (:`Released`
    (`NesComponent.SetPadButtonState` _nes 0 "A" false :!label _label_4)))

(event `Key|LeftControl`
  (params (Key :type "Key Structure"))
  ;[1 1 1] Input
  (:`Pressed`
    (goto _label_3))
  (:`Released`
    (goto _label_4)))

(event `Key|Gamepad_DPad_Up`
  (params (Key :type "Key Structure"))
  (bind _nes (`self.Nes`))
  ;[1 1 1] Input
  (:`Pressed`
    (`NesComponent.SetPadButtonState` _nes 0 "UP" true :!label _label_5))
  (:`Released`
    (`NesComponent.SetPadButtonState` _nes 0 "UP" false :!label _label_6)))

(event `Key|Up`
  (params (Key :type "Key Structure"))
  ;[1 1 1] Input
  (:`Pressed`
    (goto _label_5))
  (:`Released`
    (goto _label_6)))

(event `Key|Gamepad_DPad_Left`
  (params (Key :type "Key Structure"))
  (bind _nes (`self.Nes`))
  ;[1 1 1] Input
  (:`Pressed`
    (`NesComponent.SetPadButtonState` _nes 0 "LEFT" true :!label _label_7))
  (:`Released`
    (`NesComponent.SetPadButtonState` _nes 0 "LEFT" false :!label _label_8)))

(event `Key|Left`
  (params (Key :type "Key Structure"))
  ;[1 1 1] Input
  (:`Pressed`
    (goto _label_7))
  (:`Released`
    (goto _label_8)))

(event `Key|Gamepad_DPad_Right`
  (params (Key :type "Key Structure"))
  (bind _nes (`self.Nes`))
  ;[1 1 1] Input
  (:`Pressed`
    (`NesComponent.SetPadButtonState` _nes 0 "RIGHT" true :!label _label_9))
  (:`Released`
    (`NesComponent.SetPadButtonState` _nes 0 "RIGHT" false :!label _label_10)))

(event `Key|Gamepad_DPad_Down`
  (params (Key :type "Key Structure"))
  (bind _nes (`self.Nes`))
  ;[1 1 1] Input
  (:`Pressed`
    (`NesComponent.SetPadButtonState` _nes 0 "DOWN" true :!label _label_11))
  (:`Released`
    (`NesComponent.SetPadButtonState` _nes 0 "DOWN" false :!label _label_12)))

(event `Key|Down`
  (params (Key :type "Key Structure"))
  ;[1 1 1] Input
  (:`Pressed`
    (goto _label_11))
  (:`Released`
    (goto _label_12)))

(event `Key|Right`
  (params (Key :type "Key Structure"))
  ;[1 1 1] Input
  (:`Pressed`
    (goto _label_9))
  (:`Released`
    (goto _label_10)))

(event `Key|Gamepad_Special_Left`
  (params (Key :type "Key Structure"))
  (bind _nes (`self.Nes`))
  ;[1 1 1] Input
  (:`Pressed`
    (`NesComponent.SetPadButtonState` _nes 0 "SELECT" true :!label _label_13))
  (:`Released`
    (`NesComponent.SetPadButtonState` _nes 0 "SELECT" false :!label _label_14)))

(event `Key|LeftShift`
  (params (Key :type "Key Structure"))
  ;[1 1 1] Input
  (:`Pressed`
    (goto _label_13))
  (:`Released`
    (goto _label_14)))

(event `Key|Gamepad_FaceButton_Left`
  (params (Key :type "Key Structure"))
  (bind _nes (`self.Nes`))
  ;[1 1 1] Input
  (:`Pressed`
    (`NesComponent.SetPadButtonState` _nes 0 "B" true :!label _label_15))
  (:`Released`
    (`NesComponent.SetPadButtonState` _nes 0 "B" false :!label _label_16)))

(event `Key|LeftAlt`
  (params (Key :type "Key Structure"))
  ;[1 1 1] Input
  (:`Pressed`
    (goto _label_15))
  (:`Released`
    (goto _label_16)))

(event `Key|Escape`
  (params (Key :type "Key Structure"))
  ;[1 1 1] Input
  ;;[0 0.1597 1] Release control back to pawn
  (:`Pressed`
    (`self.SetPlayer` null)))

(event `Key|R`
  (params (Key :type "Key Structure"))
  (bind _nes (`self.Nes`))
  ;[1 1 1] Input
  ;;[0 0.1597 1] Toggle use render thread
  (:`Pressed`
    (`NesComponent.SetUpdateVideoOnRenderThread` _nes (not (`NesComponent.bUpdateVideoOnRenderThread` _nes)))))

(fn `SetPlayer`
  (params (Player :type "PlayerController Object Reference"))
  (`/Engine/EditorBlueprintResources/StandardMacros.IsValid` Player
    (:`Is Valid`
      (set `self.CurrentPlayer` (`local.Player`))
      (`PlayerController.SetViewTargetWithBlend` (`local.Player`) self 0.25 "VTBlend_Linear" 0.0 false)
      (`self.EnableInput` (`local.Player`)))
    (:`Is Not Valid`
      (bind _currentplayer (`self.CurrentPlayer`)
        (:`then`
          (`PlayerController.SetViewTargetWithBlend` _currentplayer (`Controller.K2_GetPawn` _currentplayer) 0.25 "VTBlend_Linear" 0.0 false)
          (`self.DisableInput` (`self.CurrentPlayer`))
          (set `self.CurrentPlayer` null))
        (:`else`)))))

(fn `UserConstructionScript`)